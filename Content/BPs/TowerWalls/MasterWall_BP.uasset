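; Base wall piece for tower placement in a top-down game, with a clickable pedestal that can hold one tower.
; Clicks are forwarded to the player's TopDownCharacter, cached on BeginPlay.
; Towers are added and removed by swapping the Tower child actor's class.
; Pedestal material slots show selection highlight, only when empty, and the tower's level as up to three emissive lights.
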(event `self.ReceiveBeginPlay`
  (bind _astop_down_controller (cast `/Game/BPs/TopDownController` (`GameplayStatics.GetPlayerController` 0)))
  (set `self.Controller Reference` _astop_down_controller)
  (bind _astop_down_character (cast `/Game/BPs/TopDownCharacter` (`Controller.K2_GetPawn` _astop_down_controller)))
  (set `self.Player Character Reference` _astop_down_character))

(event `self.Pedestal.OnClicked`
  (params (TouchedComponent :type "PrimitiveComponent Object Reference") (ButtonPressed :type "Key Structure"))
  (`/Game/BPs/TopDownCharacter.On Pedestal Click` (`self.Player Character Reference`) self))

(fn `Add Tower`
  (params (`Tower Class` :type "/Game/BPs/Towers/Master_Tower_BP Class Reference"))
  (`ChildActorComponent.SetChildActorClass` (`self.Tower`) `Tower Class`)
  (set `self.Tower Reference` (cast `/Game/BPs/Towers/Master_Tower_BP` (`ChildActorComponent.ChildActor` (`self.Tower`)) :!pure true)))

(fn `Remove Tower`
  (`ChildActorComponent.SetChildActorClass` (`self.Tower`) null)
  (set `self.Tower Reference` null)
  (`KismetSystemLibrary.PrintString` "Hello")
  (return))

(fn `Toggle Pedestal Hightlight`
  (params (`True - on / False - off` :type Boolean))
  (if `True - on / False - off`
    (`/Engine/EditorBlueprintResources/StandardMacros.IsValid` (`ChildActorComponent.ChildActor` (`self.Tower`))
      (:`Is Not Valid`
        (`PrimitiveComponent.SetMaterial` (`self.Pedestal`) 0 "/Game/Materials/Selection_MAT.Selection_MAT")))
    (else
      (`PrimitiveComponent.SetMaterial` (`self.Pedestal`) 0 "/Game/Materials/Default_MAT.Default_MAT"))))

(fn `Update Level Light`
  (bind _tower_reference (`self.Tower Reference`))
  (if (or (== (`/Game/BPs/Towers/Master_Tower_BP.Tower Level` _tower_reference) 0) (not (`KismetSystemLibrary.IsValid` _tower_reference)))
    (for _index (range 1 4)
      (`PrimitiveComponent.SetMaterial` (`self.Pedestal`) _index "/Game/Materials/WhiteLight_MAT.WhiteLight_MAT"))
    (else
      (for _index_2 (range 1 4)
        (if (<= _index_2 (`/Game/BPs/Towers/Master_Tower_BP.Tower Level` (`self.Tower Reference`)))
          (`PrimitiveComponent.SetMaterial` (`self.Pedestal`) _index_2 "/Game/Materials/WhiteLight_Emissive_MAT.WhiteLight_Emissive_MAT")
          (else
            (`PrimitiveComponent.SetMaterial` (`self.Pedestal`) _index_2 "/Game/Materials/WhiteLight_MAT.WhiteLight_MAT")))))))

(fn `UserConstructionScript`)