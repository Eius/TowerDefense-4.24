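; CornerWall_BP is a corner tower wall piece whose blue light follows a controller's intensity.
; On BeginPlay, after the parent logic, it creates a dynamic instance of BlueLight_MAT on one material slot of the Wall mesh.
; Every Tick it copies Intensity from ControllerReference into that material's Intensity parameter.
; The construction script only calls the parent.
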(event `self.ReceiveBeginPlay`
  (`parent.ReceiveBeginPlay`)
  (bind _returnvalue (`PrimitiveComponent.CreateDynamicMaterialInstance` (`self.Wall`) 4 "/Game/Materials/BlueLight_MAT.BlueLight_MAT" "None"))
  (set `self.Big Blue Light` _returnvalue))

(event `self.ReceiveTick`
  (params (DeltaSeconds :type "Float (single-precision)"))
  (`MaterialInstanceDynamic.SetScalarParameterValue` (`self.Big Blue Light`) "Intensity" (`/Game/BPs/TopDownController.Intensity` (`self.Controller Reference`))))

(fn `UserConstructionScript`
  (`parent.UserConstructionScript`))