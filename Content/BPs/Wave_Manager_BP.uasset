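; Wave manager that spawns timed waves of enemy AI along a path of placed waypoints.
; On BeginPlay it sorts AI_Point_BP actors by Index into AIPath, takes the first as spawn location, and starts the countdown after a delay.
; At zero, SpawnWave reads the current wave's Waves_DT row and spawns EnemyAI_BP one by one at its interval, passing path and stats.
; Tick watches FinishedSpawning to restart the countdown for the next wave.
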(event `self.ReceiveBeginPlay`
  (`self.Create AI Path`)
  (`self.Set AI Spawn Location`
    (:`Out`
      (`KismetSystemLibrary.Delay` (`self.Start Game Delay`))
      (`self.Start Spawning Waves`))))

(event `Start Spawning Waves`
  (bind _returnvalue (`KismetSystemLibrary.K2_SetTimerDelegate` (delegate `Decrement from Timer`) 1.0 true :!label _label))
  (set `self.Timer Handle` _returnvalue)
  (set `self.Finished Spawning?` false))

(event `self.ReceiveTick`
  (params (DeltaSeconds :type "Float (single-precision)"))
  (if (`self.Finished Spawning?`)
    (set `self.Time to Spawn New Wave` 20)
    (goto _label)))

(event `Decrement from Timer`
  (bind _result (`/Engine/EditorBlueprintResources/StandardMacros.DecrementInt` (`self.Time to Spawn New Wave`))
    (:`  `
      (if (== _result 0)
        (`KismetSystemLibrary.K2_ClearAndInvalidateTimerHandle` (`self.Timer Handle`))
        (`self.Spawn Wave`
          (:`Out`
            (`/Engine/EditorBlueprintResources/StandardMacros.IncrementInt` (`self.Wave Number`)
              (:`  `
                (set `self.Finished Spawning?` true)))))))))

(fn `Create AI Path`
  (locals (Temp_Array :type "Array of /Game/BPs/AI_Point_BP Object Reference") (`Target Index` :type Integer) (Sorted_Array :type "Array of /Game/BPs/AI_Point_BP Object Reference"))
  (bind _outactors (`GameplayStatics.GetAllActorsOfClass` "/Game/BPs/AI_Point_BP.AI_Point_BP_C"))
  (bind _output_get (set `local.Temp_Array` _outactors))
  (for (_array_element _array_index) _output_get :!label _label
    (if (== (`/Game/BPs/AI_Point_BP.Index` _array_element) (`local.Target Index`))
      (`KismetArrayLibrary.Array_Add` (`local.Sorted_Array`) _array_element)
      (`/Engine/EditorBlueprintResources/StandardMacros.IncrementInt` (`local.Target Index`)
        (:`  `
          (`KismetArrayLibrary.Array_Remove` (`local.Temp_Array`) _array_index)
          (break)))))
  (if (`KismetArrayLibrary.Array_IsValidIndex` (`local.Temp_Array`))
    (goto _label)
    (else
      (set `self.AI_Path` (`local.Sorted_Array`))
      (return))))

(fn `UserConstructionScript`)