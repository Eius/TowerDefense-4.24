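; Homing rocket projectile fired by the Rocket Tower, damaging enemies on impact and nearby ones with splash.
; It launches along the tower's spawn point forward vector, then after a short delay a looping timer keeps updating homing toward the target while spawning trail particles.
; Hitting an enemy deals full damage, then explodes for half damage to others in an enlarged sphere.
; Floor hits or a lifetime timeout also explode and destroy it.
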(event `self.ReceiveBeginPlay`
  (bind _target (`self.Target`))
  (bind _projectilemovement (`self.ProjectileMovement`))
  (bind _projectilemovement_2 (`self.ProjectileMovement`))
  (bind (_returnvalue_x _returnvalue_y _returnvalue_z) (`KismetMathLibrary.BreakVector` (`SceneComponent.GetForwardVector` (`/Game/BPs/Towers/Rocket_Tower.Projectile Spawn Placeholder` (cast `/Game/BPs/Towers/Rocket_Tower` (`self.Tower`) :!pure true)))))
  (`KismetSystemLibrary.K2_SetTimerDelegate` (delegate `Custom Tick`) 0.2 true)
  (set `MovementComponent.Velocity` (* (`KismetMathLibrary.MakeVector` _returnvalue_x _returnvalue_y _returnvalue_z) (1800.0 1800.0 1800.0)) (`self.ProjectileMovement`))
  (`KismetSystemLibrary.Delay` 0.22)
  (`|ExecutionSequence`
    (:`then_0`
      (`KismetSystemLibrary.Delay` 3.0)
      (`self.Explode` (`self.Target`))
      (`self.K2_DestroyActor`))
    (:`then_1`
      (goto _label :!via `Open`))))

(event `Custom Tick`
  (bind _target (`self.Target`))
  (bind _projectilemovement (`self.ProjectileMovement`))
  (bind _projectilemovement_2 (`self.ProjectileMovement`))
  (`self.TrailParticle`)
  (`/Engine/EditorBlueprintResources/StandardMacros.Gate` true :!label _label
    (:`Exit`
      (`/Engine/EditorBlueprintResources/StandardMacros.IsValid` _target
        (:`Is Valid`
          (set `ProjectileMovementComponent.HomingTargetComponent` (`/Game/BPs/Enemy/EnemyAI_BP.Cube` _target) _projectilemovement_2)
          (set `ProjectileMovementComponent.bIsHomingProjectile` true _projectilemovement_2))
        (:`Is Not Valid`
          (set `ProjectileMovementComponent.HomingTargetComponent` null _projectilemovement)
          (set `ProjectileMovementComponent.bIsHomingProjectile` false _projectilemovement))))))

(event `self.Cube.OnComponentBeginOverlap`
  (params (OverlappedComponent :type "PrimitiveComponent Object Reference") (OtherActor :type "Actor Object Reference") (OtherComp :type "PrimitiveComponent Object Reference") (OtherBodyIndex :type Integer) (bFromSweep :type Boolean) (SweepResult :type "HitResult Structure (by ref)"))
  (bind _tower (`self.Tower`))
  (bind _asenemy_ai_bp (cast `/Game/BPs/Enemy/EnemyAI_BP` OtherActor)
    (:`then`
      (message `/Game/BPs/Damage_Interface.Deal Damage` _asenemy_ai_bp (`/Game/BPs/Towers/Master_Tower_BP.Damage` _tower) _tower)
      (`self.Explode` _asenemy_ai_bp)
      (`self.K2_DestroyActor`))
    (:`CastFailed`
      (cast `/Game/BPs/TowerWalls/Floor_BP` OtherActor)
      (`self.Explode` null)
      (`self.K2_DestroyActor`))))

(fn `Explode`
  (params (`Target to Ignore` :type "/Game/BPs/Enemy/EnemyAI_BP Object Reference"))
  (bind _tower (`self.Tower`))
  (`GameplayStatics.SpawnEmitterAtLocation` "/Game/Particles/BigExplosion_Particle1.BigExplosion_Particle1" (`self.K2_GetActorLocation`))
  (`SphereComponent.SetSphereRadius` (`self.Sphere`) 400.0 true)
  (for _array_element (`PrimitiveComponent.GetOverlappingActors` (`self.Sphere`) "/Game/BPs/Enemy/EnemyAI_BP.EnemyAI_BP_C")
    (if (not (== `Target to Ignore` _array_element))
      (message `/Game/BPs/Damage_Interface.Deal Damage` _array_element (/ (`/Game/BPs/Towers/Master_Tower_BP.Damage` _tower) 2.0) _tower)))
  (return))

(fn `TrailParticle`
  (`GameplayStatics.SpawnEmitterAtLocation` "/Game/Particles/RocketTrail_P.RocketTrail_P" (`self.K2_GetActorLocation`) (struct) (0.5 0.5 0.5))
  (return))

(fn `UserConstructionScript`)