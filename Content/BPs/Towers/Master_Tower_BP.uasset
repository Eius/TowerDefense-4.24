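; Base tower Blueprint that attacks AI enemies inside its capsule radius, with an empty CustomAttack event as the attack hook.
; Loads stats from Towers_DT, then a fast looping timer picks first or last target and runs a repeating attack timer.
; Untargeted towers fire CustomAttack once; the target-in-radius mode only checks, without attacking.
; Level changes update the parent wall pedestal's light, and clicking the mesh asks it to remove the tower.
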(event `self.ReceiveBeginPlay`
  (`self.Set Stats`)
  (`KismetSystemLibrary.K2_SetTimerDelegate` (delegate `Custom Tick`) 0.01 true)
  (set `self.Owning Pedestal Reference` (cast `/Game/BPs/TowerWalls/MasterWall_BP` (`self.GetParentActor`) :!pure true)))

(event `Custom Attack`
  (params (`Target to attack` :type "/Game/BPs/Enemy/AI_Master_Character Object Reference")))

(event `Custom Tick`
  (if (`self.NeedSpecificTargetToAttack?`)
    (bind _target_in_radius_ (`self.Target Enemy (with targeting enum)`)
      (:`Out`
        (if _target_in_radius_
          (`/Engine/EditorBlueprintResources/StandardMacros.DoOnce` false :!label _label
            (:`Completed`
              (`self.Attack`)
              (bind _returnvalue (`KismetSystemLibrary.K2_SetTimerDelegate` (delegate `Attack`) (`self.Attack Speed`) true))
              (set `self.Attack Timer Handle` _returnvalue)))
          (else
            (`KismetSystemLibrary.K2_ClearAndInvalidateTimerHandle` (`self.Attack Timer Handle`))
            (goto _label :!via `Reset`)))))
    (elif (`self.NeedTargetInRadius?`)
      (bind _target_in_radius__2 (`self.Check for Any Valid Target`)
        (:`Out`
          (if _target_in_radius__2
            _)))
      (else
        (`/Engine/EditorBlueprintResources/StandardMacros.DoOnce` false
          (:`Completed`
            (`self.Custom Attack` null)))))))

(event `Attack`
  (bind _target (`self.Target`))
  (`/Engine/EditorBlueprintResources/StandardMacros.IsValid` _target
    (:`Is Valid`
      (`self.Custom Attack` _target)
      (`KismetSystemLibrary.Delay` (- (`self.Attack Speed`) 0.01)))))

(event `self.Capsule.OnComponentBeginOverlap`
  (params (OverlappedComponent :type "PrimitiveComponent Object Reference") (OtherActor :type "Actor Object Reference") (OtherComp :type "PrimitiveComponent Object Reference") (OtherBodyIndex :type Integer) (bFromSweep :type Boolean) (SweepResult :type "HitResult Structure (by ref)"))
  (bind _asai_master_character (cast `/Game/BPs/Enemy/AI_Master_Character` OtherActor))
  (`KismetArrayLibrary.Array_Add` (`self.Enemies in radius`) _asai_master_character))

(event `self.Capsule.OnComponentEndOverlap`
  (params (OverlappedComponent :type "PrimitiveComponent Object Reference") (OtherActor :type "Actor Object Reference") (OtherComp :type "PrimitiveComponent Object Reference") (OtherBodyIndex :type Integer))
  (bind _asai_master_character (cast `/Game/BPs/Enemy/AI_Master_Character` OtherActor))
  (`KismetArrayLibrary.Array_RemoveItem` (`self.Enemies in radius`) _asai_master_character))

(event `self.TowerMesh.OnClicked`
  (params (TouchedComponent :type "PrimitiveComponent Object Reference") (ButtonPressed :type "Key Structure"))
  (`/Game/BPs/TowerWalls/MasterWall_BP.Remove Tower` (`self.Owning Pedestal Reference`)))

(fn `Add Level`
  (bind _tower_level (`self.Tower Level`))
  (if (not (== _tower_level 3))
    (`/Engine/EditorBlueprintResources/StandardMacros.IncrementInt` _tower_level
      (:`  `
        (`/Game/BPs/TowerWalls/MasterWall_BP.Update Level Light` (`self.Owning Pedestal Reference`))))))

(fn `Check for Last Target`
  (returns (`EnemiesInRadius?` :type Boolean) (Target :type "/Game/BPs/Enemy/AI_Master_Character Object Reference"))
  (locals (localBool :type Boolean) (localTarget :type "/Game/BPs/Enemy/AI_Master_Character Object Reference"))
  (set `local.localBool` false)
  (for _array_element (`self.Enemies in radius`)
    (`/Engine/EditorBlueprintResources/StandardMacros.IsValid` _array_element
      (:`Is Valid`
        (set `local.localBool` true)
        (set `local.localTarget` _array_element))))
  (return (`local.localBool`) (`local.localTarget`)))

(fn `Decrease Level`
  (bind _tower_level (`self.Tower Level`))
  (if (not (== _tower_level 0))
    (`/Engine/EditorBlueprintResources/StandardMacros.DecrementInt` _tower_level
      (:`  `
        (`/Game/BPs/TowerWalls/MasterWall_BP.Update Level Light` (`self.Owning Pedestal Reference`))))))

(fn `Set Stats`
  (bind _returnvalue (`|GetDataTableRow` "/Game/BPs/DataTables/Towers_DT.Towers_DT" (`self.Tower Name`))
    (:`then`
      (set `self.Attack Speed` (break `/Game/BPs/Structs/Tower_Sctruct` _returnvalue))
      (set `self.Damage` (`.Damage_29_9C1C12A848A50F1551D9169B9B25F8B4` (break `/Game/BPs/Structs/Tower_Sctruct` _returnvalue)))
      (set `self.NeedSpecificTargetToAttack?` (`.NeedSpecificTargettoAttack?overridestargetinradiusboolean_36_FDF0B1204399AAAD8E1329BB79D0B124` (break `/Game/BPs/Structs/Tower_Sctruct` _returnvalue)))
      (set `self.NeedTargetInRadius?` (`.NeedTargetinRadius?bothbooleansfalseattacksperpetually_39_3D24ECC44DD6532CC367639D8CDFDB6F` (break `/Game/BPs/Structs/Tower_Sctruct` _returnvalue)))
      (return))))

(fn `UserConstructionScript`)