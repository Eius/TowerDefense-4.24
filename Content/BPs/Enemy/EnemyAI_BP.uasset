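; Enemy pawn for a wave-based game that follows AIPath actors via chained AI MoveTo calls and pays a bounty when killed.
; SetStats derives health, bounty, speed and damage from wave data.
; Debuffs refresh their timestamp when reapplied and expire through a 0.2-second timer instead of Tick.
; Only movement-speed debuffs change stats, adjusting FloatingPawnMovement speed; damage reduction and stun are empty stubs.
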(event `/Game/BPs/Damage_Interface.Deal Damage`
  (params (Damage :type "Float (single-precision)") (Instigator :type "/Game/BPs/Towers/Master_Tower_BP Object Reference"))
  ;[1 1 1] Take Damage
  (bind _output_get (set `self.ActualHealth` (- (`self.ActualHealth`) Damage)))
  (if (<= _output_get 0.0)
    (`/Game/BPs/TopDownController.Add Money` (`self.Controller Reference`) (`self.Bounty`))
    (`self.K2_DestroyActor`)))

(event `self.ReceiveBeginPlay`
  ;[1 1 1] Begin Play
  (`self.Set HP Widget`
    (:`Out`
      (`self.Start Custom Tick`)
      (`self.AI_PathLoop`))))

(event `Start Custom Tick`
  ;[1 1 1] Custom Tick
  (`KismetSystemLibrary.K2_SetTimerDelegate` (delegate `Custom Tick`) 0.2 true))

(event `Custom Tick`
  ;[1 1 1] Custom Tick
  (`self.Check Expired Debuffs`))

(event `Event Add Debuff`
  (params (Debuff :type "/Game/BPs/Structs/Debuff_Struct Structure"))
  ;[1 1 1] Add Debuff
  (`self.Add Debuff` Debuff
    (:`Out`
      (`self.Apply Debuff` Debuff))))

(fn `Set Stats`
  (params (`Wave Stats Struct` :type "/Game/BPs/Structs/Wave_Struct Structure") (`Wave Number` :type Integer))
  (bind (_basebounty _basehealth) (break `/Game/BPs/Structs/Wave_Struct` `Wave Stats Struct`))
  (bind _wave_number (`local.Wave Number`))
  (bind (_wave_stats_struct_basebounty _wave_stats_struct_basehealth _wave_stats_struct_speed _wave_stats_struct_damage) (break `/Game/BPs/Structs/Wave_Struct` (`local.Wave Stats Struct`)))
  (bind _health (`self.Calculate Health` _basehealth _wave_number))
  (set `self.Bounty` (`self.Calculate Bounty` _basebounty _wave_number))
  (set `self.ActualHealth` _health)
  (set `self.MaxHealth` _health)
  (bind _output_get (set `self.Base Movement Speed` _wave_stats_struct_speed))
  (set `FloatingPawnMovement.MaxSpeed` _output_get (`self.FloatingPawnMovement`))
  (set `self.Damage` _wave_stats_struct_damage)
  (return))

(fn `UserConstructionScript`)