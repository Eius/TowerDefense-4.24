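; GradientTestPlane_BP is a test actor that previews a gradient material driven by values from the TopDownController.
; On BeginPlay it creates a dynamic instance of Gradient_MAT on its mesh, caches the controller and prints the Sphere's base scale.
; Each tick it copies the controller's Fill value into the material's Fill parameter.
; Unconnected nodes would also drive Lerp and Intensity and scale two spheres by Fill.
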(event `self.ReceiveBeginPlay`
  (bind _returnvalue (`PrimitiveComponent.CreateDynamicMaterialInstance` (`self.StaticMeshComponent`) 0 "/Game/Materials/Gradient_MAT.Gradient_MAT" "None"))
  (set `self.Dynamic Material` _returnvalue)
  (bind _astop_down_controller (cast `/Game/BPs/TopDownController` (`GameplayStatics.GetPlayerController` 0)))
  (set `self.Controller` _astop_down_controller)
  (bind _output_get (set `self.SphereBaseScale` (`SceneComponent.K2_GetComponentScale` (`self.Sphere`))))
  (`KismetSystemLibrary.PrintString` (`KismetStringLibrary.Conv_VectorToString` _output_get)))

(event `self.ReceiveTick`
  (params (DeltaSeconds :type "Float (single-precision)"))
  (`MaterialInstanceDynamic.SetScalarParameterValue` (`self.Dynamic Material`) "Fill" (`/Game/BPs/TopDownController.Fill` (`self.Controller`))))

(fn `UserConstructionScript`)